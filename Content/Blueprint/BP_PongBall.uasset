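; BP_PongBall is the ball actor for a Pong game, moved by physics impulses on its Sphere component.
; On BeginPlay it launches along +X after a one-second delay and binds to the GM_Pong game mode's EdResetBall dispatcher.
; When that dispatcher fires, it moves to a fixed position without clearing velocity, waits a second, then applies a far weaker +X impulse than the opening launch.
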(event `self.ReceiveBeginPlay`
  (`|ExecutionSequence`
    (:`then_0`
      (`KismetSystemLibrary.Delay` 1.0)
      (`PrimitiveComponent.AddImpulse` (`self.Sphere`) (2000.0 0.0 0.0) "None" false))
    (:`then_1`
      (bind _asgm_pong (cast `/Game/System/GM_Pong` (`GameplayStatics.GetGameMode`)))
      (bind _output_get (set `self.GmRef` _asgm_pong))
      (add `/Game/System/GM_Pong.EdResetBall` _output_get (delegate `EdResetBall_Event_0`)))))

(event `EdResetBall_Event_0`
  (`self.K2_SetActorRelativeLocation` (0.0 0.0 20.0))
  (`KismetSystemLibrary.Delay` 1.0)
  (`PrimitiveComponent.AddImpulse` (`self.Sphere`) (20.0 0.0 0.0) "None" false))

(fn `UserConstructionScript`)