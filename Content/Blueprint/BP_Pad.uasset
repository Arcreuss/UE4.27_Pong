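; Player-controlled paddle pawn for a Pong game.
; The VerticalMovement axis feeds a scaled world-Y input vector into its floating pawn movement component.
; The Reset action destroys the BP_PongBall found in the level and spawns a replacement at the SpawnBall transform.
; BeginPlay caches the GM_Pong game mode, though nothing in these graphs uses that reference.
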(event `self.ReceiveBeginPlay`
  (bind _asgm_pong (cast `/Game/System/GM_Pong` (`GameplayStatics.GetGameMode`)))
  (set `self.GmRef` _asgm_pong))

(event `InputAction|Reset`
  (params (Key :type "Key Structure"))
  (:`Pressed`
    (bind _returnvalue (`GameplayStatics.GetActorOfClass` "/Game/Blueprint/BP_PongBall.BP_PongBall_C"))
    (`self.K2_DestroyActor` _returnvalue)
    (`|SpawnActorFromClass` "/Game/Blueprint/BP_PongBall.BP_PongBall_C" (`self.SpawnBall`) "Undefined" "OverrideRootScale" null null)))

(event `InputAxis|VerticalMovement`
  (params (AxisValue :type "Float (single-precision)"))
  (`PawnMovementComponent.AddInputVector` (`self.FloatingPawnMovementPad`) (`KismetMathLibrary.MakeVector` 0.0 (* AxisValue 10.0)) false))

(fn `UserConstructionScript`)